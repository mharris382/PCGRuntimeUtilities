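; PCGGenHitTrigger is an actor component that listens for physics hits on its owner, apparently as a trigger for PCG generation, though it only prints debug output.
; On BeginPlay it finds the owner's first primitive component carrying TriggerComponentTag and binds to its hit event.
; Each hit prints the components and actor involved, plus the hit item and element index, which can identify individual instances or elements.
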(event Custom|OnHit
  (params (HitComponent :type Primitive%20Component%20Object%20Reference) (OtherActor :type Actor%20Object%20Reference) (OtherComp :type Primitive%20Component%20Object%20Reference) (NormalImpulse :type Vector) (Hit :type Hit%20Result%20Structure%20%28by%20ref%29))
  (bind (_bblockinghit _binitialoverlap _time _distance _location _impactpoint _normal _impactnormal _physmat _hitactor _hitcomponent _hitbonename _bonename _hititem _elementindex) (Collision|BreakHitResult Hit))
  (Development|PrintText (Utilities|Text|FormatText "HitComponent {0} 
OtherActor {1} 
Other Comp {2} 
Hit Item {3} 
Element Index {4}" (Utilities|GetDisplayName HitComponent) (Utilities|GetDisplayName OtherActor) (Utilities|GetDisplayName OtherComp) _hititem _elementindex) true true "(R=1.000000,G=0.353617,B=0.001269,A=1.000000)"))

(event EventBeginPlay
  (bind _returnvalue (Components|GetOwner))
  (bind _triggercomponenttag (Variables|Default|GetTriggerComponentTag))
  (bind _returnvalue_2 (Actor|GetComponentsbyTag _returnvalue "/Script/Engine.PrimitiveComponent" _triggercomponenttag))
  (if (Utilities|Array|IsNotEmpty _returnvalue_2)
    (Collision|BindEventtoOnComponentHit (Utilities|Array|Get(acopy) _returnvalue_2) (delegate Custom|OnHit))))

(event EventTick
  (params (DeltaSeconds :type Float%20%28single-precision%29)))